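; BP_Ragdoll is a ragdoll body that periodically emits radio chatter from its position.
; On BeginPlay it disables capsule collision, simulates physics on all mesh bodies and picks a random delay.
; Tick accumulates delta time, then plays an attenuated US radio sound at the actor's location and picks a new random delay.
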(event EventBeginPlay
  (Collision|SetCollisionEnabled (Variables|Collision|GetCapsuleComponent) "NoCollision")
  (Class|SkeletalMeshComponent|SetAllBodiesSimulatePhysics (Variables|Character|GetMesh) true)
  (Variables|Default|SetradioTime (Math|Random|RandomFloatinRange 1e+01 6e+01)))

(event Collision|EventActorBeginOverlap
  (params (OtherActor :type Actor%20Object%20Reference)))

(event EventTick
  (params (DeltaSeconds :type Float%20%28single-precision%29))
  (if (> (Variables|Default|Gettime) (Variables|Default|GetradioTime))
    (Variables|Default|Settime 0.0)
    (Variables|Default|SetradioTime (Math|Random|RandomFloatinRange 1e+01 6e+01))
    (Audio|PlaySoundatLocation "/Game/Sounds/SE/SystemSE/USA_radio_am2.USA_radio_am2" (Transformation|GetActorLocation) "0, 0, 0" 1.0 1.0 0.0 "/Game/Sounds/GeneralSoundAttenuation.GeneralSoundAttenuation")
    (else
      (Variables|Default|Settime (+ (Variables|Default|Gettime) (Utilities|Time|GetWorldDeltaSeconds))))))

(fn ConstructionScript)