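; Player character for a first-person stealth horror game whose enemies are hidden from the main camera, leaving the battery-limited smartphone camera to reveal them.
; SwitchCamera raises or lowers the animated phone, toggling its render target; no-collider walls are hidden from that capture.
; A forward trace selects chargers, lockers, keys, switches or the goal for interaction.
; Tick reports running noise and polls AI controllers for discovery FOV pulses; enemy contact triggers game over.
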(event EventBeginPlay
  ;[1 1 1] BP_CameraUIの取得
  (bind _returnvalue (UserInterface|CreateWidget "/Game/Blueprints/Sekine/UI/MainCamera.MainCamera_C"))
  (bind _output_get (Variables|Default|SetMainUI _returnvalue))
  (UserInterface|Viewport|AddtoViewport _output_get 0)
  (bind _returnvalue_2 (UserInterface|CreateWidget "/Game/Blueprints/Sekine/UI/BP_MainUI.BP_MainUI_C"))
  (bind _output_get_2 (Variables|Default|SetMenu _returnvalue_2))
  (Default|SetPlayer _output_get_2 self)
  ;[1 1 1] Enemyの取得
  (bind _outactors (Actor|GetAllActorsOfClass "/Game/Blueprints/Reito/Enemy/AI_Beta/BetaEnemy.BetaEnemy_C"))
  (for _array_element _outactors
    (bind _asbeta_enemy (Utilities|Casting|CastToBetaEnemy _array_element))
    (CallFunction|AddMainCameraHiddenActor _asbeta_enemy))
  (bind _outactors_2 (Actor|GetAllActorsOfClass "/Game/Blueprints/Reito/Enemy/AI_Beta/Enemy2.Enemy2_C"))
  (for _array_element_2 _outactors_2
    (bind _asenemy_2 (Utilities|Casting|CastToEnemy2 _array_element_2))
    (CallFunction|AddMainCameraHiddenActor _asenemy_2))
  (Variables|Default|SetplayerController (Game|GetPlayerController 0))
  (bind _outactors_3 (Actor|GetAllActorsOfClass "/Game/Blueprints/Reito/Architecture/BP_NoColliderWall.BP_NoColliderWall_C"))
  (for _array_element_3 _outactors_3
    (Utilities|Array|Add (Variables|/Script/Engine.SceneCaptureComponent|GetHiddenActors (Variables|Default|GetSmartphoneCamera)) _array_element_3))
  (bind _outactors_4 (Actor|GetAllActorsOfClass "/Game/Blueprints/Reito/Enemy/AI_Beta/Beta_AI_CON.Beta_AI_CON_C"))
  (for _array_element_4 _outactors_4
    (bind _asbeta_ai_con (Utilities|Casting|CastToBeta_AI_CON _array_element_4))
    (Utilities|Array|Add (Variables|Default|GetAI_CON) _asbeta_ai_con)
    (Utilities|Array|Add (Variables|Default|Getfound) false)
    (Utilities|Array|Add (Variables|Default|GetbeforeFound) false))
  (bind _outactors_5 (Actor|GetAllActorsOfClass "/Game/Blueprints/Reito/Enemy/AI_Beta/Enemy2_AI_CON.Enemy2_AI_CON_C"))
  (for _array_element_5 _outactors_5
    (bind _asenemy_2_ai_con (Utilities|Casting|CastToEnemy2_AI_CON _array_element_5))
    (Utilities|Array|Add (Variables|Default|GetAI2_CON) _asenemy_2_ai_con)
    (Utilities|Array|Add (Variables|Default|Getfound) false)
    (Utilities|Array|Add (Variables|Default|GetbeforeFound) false))
  (Audio|Components|Audio|Stop (Variables|Default|GetfootSteps_Cue)))

(event Collision|EventHit
  (params (MyComp :type Primitive%20Component%20Object%20Reference) (Other :type Actor%20Object%20Reference) (OtherComp :type Primitive%20Component%20Object%20Reference) (bSelfMoved :type Boolean) (HitLocation :type Vector :default "0, 0, 0") (HitNormal :type Vector :default "0, 0, 0") (NormalImpulse :type Vector :default "0, 0, 0") (Hit :type Hit%20Result%20Structure%20%28by%20ref%29))
  (switch Utilities|FlowControl|Switch|SwitchonEPlayerCondition (Variables|Default|Getcondition)
    (:Normal
      (Utilities|Casting|CastToBetaEnemy Other
        (:then
          _)
        (:CastFailed
          (Utilities|Casting|CastToEnemy2 Other)))
      (Game|OpenLevel(byName) "GameOverLevel"))))

(event EventTick
  (params (DeltaSeconds :type Float%20%28single-precision%29))
  ;[1 1 1] 走っていたらノイズを発生させる
  (if (> (Class|MovementComponent|GetMaxSpeed (Variables|Character|GetCharacterMovement)) (Variables|Default|GetwalkSpeed))
    (Class|AISenseHearing|ReportNoiseEvent (Transformation|GetActorLocation) 1.0 self 0.0 "None"))
  ;[1 1 1] プレイヤーの前1m以内にあるアクタの取得
  (bind (_outhit _returnvalue) (Collision|LineTraceByChannel (Transformation|GetActorLocation) (+ (Transformation|GetActorLocation) (* (Math|Vector|GetForwardVector (Variables|Default|GetCapsuleComponent)) 100)) "TraceTypeQuery1" false 0 "None"))
  (if _returnvalue
    (Variables|Default|SetfrontActor (.hitactor _outhit))
    (else
      (Variables|Default|SetfrontActor 0)))
  (if (< (Variables|Default|Getbattery) 0.0)
    (Variables|Default|Setbattery 0.0)
    (CallFunction|SwitchCamera))
  (Transformation|SetWorldRotation (Variables|Default|GetMainCamera) (Pawn|GetControlRotation (Variables|Default|GetplayerController) :!class /Script/Engine.Controller) false false)
  (for (_array_element _array_index) (Variables|Default|GetAI_CON)
    (Utilities|Array|SetArrayElem (Variables|Default|Getfound) _array_index (and (Variables|/Game/Blueprints/Reito/Enemy/AI_Beta/Beta_AI_CON.Beta_AI_CON_C|GetPlayerDiscovery _array_element) (not (Utilities|Array|Get(acopy) (Variables|Default|GetbeforeFound) _array_index))))
    (CallFunction|ChangeFOV (Variables|/Game/Blueprints/Reito/Enemy/AI_Beta/Beta_AI_CON.Beta_AI_CON_C|GetDiscoveryTiming _array_element))
    (Variables|/Game/Blueprints/Reito/Enemy/AI_Beta/Beta_AI_CON.Beta_AI_CON_C|SetDiscoveryTiming _array_element false))
  (for (_array_element_2 _array_index_2) (Variables|Default|GetAI2_CON)
    (Utilities|Array|SetArrayElem (Variables|Default|Getfound) _array_index_2 (and (Variables|/Game/Blueprints/Reito/Enemy/AI_Beta/Enemy2_AI_CON.Enemy2_AI_CON_C|GetPlayerDiscovery _array_element_2) (not (Utilities|Array|Get(acopy) (Variables|Default|GetbeforeFound) _array_index_2))))
    (CallFunction|ChangeFOV (Variables|/Game/Blueprints/Reito/Enemy/AI_Beta/Enemy2_AI_CON.Enemy2_AI_CON_C|GetDiscoveryTiming _array_element_2))
    (Variables|/Game/Blueprints/Reito/Enemy/AI_Beta/Enemy2_AI_CON.Enemy2_AI_CON_C|SetDiscoveryTiming _array_element_2 false))
  (if (not (Variables|Default|GetholdCamera))
    (if (and (Audio|Components|Audio|IsPlaying (Variables|Default|GetfootSteps_Cue)) (not (Variables|Default|GetisWalk)))
      (Audio|Components|Audio|Stop (Variables|Default|GetfootSteps_Cue))
      (elif (Math|Boolean|ANDBoolean (not (Audio|Components|Audio|IsPlaying (Variables|Default|GetfootSteps_Cue))) (Variables|Default|GetisWalk) (Variables|Default|Getsprint))
        (Audio|Components|Audio|Play (Variables|Default|GetfootSteps_Cue) 0.0)))
    (if (not (Audio|Components|Audio|IsPlaying (Variables|Default|GetSmartphone)))
      (Development|SetHiddeninGame (Variables|Default|GetSmartphone) true false))))

(event Collision|EventActorBeginOverlap
  (params (OtherActor :type Actor%20Object%20Reference))
  (Variables|Default|SetoverlapActor OtherActor))

(event Collision|EventActorEndOverlap
  (params (OtherActor :type Actor%20Object%20Reference))
  (Variables|Default|SetoverlapActor 0))

(event Input|ActionEvents|InputActionCamera
  (params (Key :type Key%20Structure))
  (:Pressed
    (switch Utilities|FlowControl|Switch|SwitchonEPlayerCondition (Variables|Default|Getcondition)
      (:Normal
        (Variables|Default|Setcamera true)
        (CallFunction|SwitchCamera)
        (Audio|Components|Audio|Stop (Variables|Default|GetfootSteps_Cue)))))
  (:Released
    (Variables|Default|Setcamera false)))

(event Input|ActionEvents|InputActionMenu
  (params (Key :type Key%20Structure))
  (bind _menu (Variables|Default|GetMenu))
  (bind _menu_2 (Variables|Default|GetMenu))
  (:Pressed
    (if (Variables|Default|GetholdCamera)
      (CallFunction|SwitchCamera)
      (elif (and (not (Audio|Components|Audio|IsPlaying (Variables|Default|GetSmartphone))) (not (Class|UserWidget|IsAnimationPlaying _menu_2 (Variables|/Game/Blueprints/Sekine/UI/BP_MainUI.BP_MainUI_C|Getmanu_animation _menu_2))))
        (Utilities|FlowControl|FlipFlop
          (:A
            (UserInterface|Viewport|AddtoViewport (Variables|Default|GetMenu) 0))
          (:B
            (UserInterface|Animation|PlayAnimation _menu (Variables|/Game/Blueprints/Sekine/UI/BP_MainUI.BP_MainUI_C|Getmanu_animation _menu) 0.0 1 "Reverse" 1.0)
            (Variables|/Game/Blueprints/Sekine/UI/BP_MainUI.BP_MainUI_C|SetwillDelete (Variables|Default|GetMenu) true)))))))

(event Input|ActionEvents|InputActionAction
  (params (Key :type Key%20Structure))
  (bind _frontactor (Variables|Default|GetfrontActor))
  (bind _frontactor_2 (Variables|Default|GetfrontActor))
  (:Pressed
    (Variables|Default|Setaction true)
    (if (and (!= (Variables|Default|GetoverlapActor) 0) (not (Variables|Default|GetholdCamera)))
      (if (!= _frontactor_2 0)
        (Variables|Default|SetactionLocation (Transformation|GetActorLocation _frontactor_2))
        (Variables|Default|SetIsAction true)
        (bind _asbp_charger (Utilities|Casting|CastToBP_Charger _frontactor)
          (:then
            (Variables|Default|SetactionActor _asbp_charger)
            (if (Variables|Default|GetcanCharge)
              (Class|MainPlayer|AddBattery (Variables|/Game/Blueprints/Sekine/BP_Charger.BP_Charger_C|GetBattery%20Value _asbp_charger))))
          (:CastFailed
            (bind _asbp_locker (Utilities|Casting|CastToBP_Locker _frontactor)
              (:then
                (Variables|Default|SetactionActor _asbp_locker)
                (Default|Enter _asbp_locker))
              (:CastFailed
                (bind _asbp_key (Utilities|Casting|CastToBP_Key _frontactor)
                  (:then
                    (Variables|Default|SetactionActor _asbp_key)
                    (CallFunction|SmartphoneAnimation "NewEnumerator2")
                    (Default|GiveKey _asbp_key self))
                  (:CastFailed
                    (bind _asbp_goal (Utilities|Casting|CastToBP_Goal _frontactor)
                      (:then
                        (Variables|Default|SetactionActor _asbp_goal)
                        (CallFunction|SmartphoneAnimation "NewEnumerator2")
                        (if (Variables|Default|GethaveKey)
                          (Game|OpenLevel(byName) "ClearLevel")))
                      (:CastFailed
                        (bind _asbp_switch (Utilities|Casting|CastToBP_Switch _frontactor))
                        (Variables|Default|SetactionActor _asbp_switch)
                        (CallFunction|SmartphoneAnimation "NewEnumerator2"))))))))))))
  (:Released
    (Variables|Default|Setaction false)
    (Variables|Default|SetactionActor 0)))

(event Input|ActionEvents|InputActionSprint
  (params (Key :type Key%20Structure))
  (:Pressed
    (Variables|Default|Setsprint true)
    (if (and (Variables|Default|GetisWalk) (not (Variables|Default|GetholdCamera)))
      (Audio|Components|Audio|Play (Variables|Default|GetfootSteps_Cue) 0.0)))
  (:Released
    (Variables|Default|Setsprint false)
    (Audio|Components|Audio|Stop (Variables|Default|GetfootSteps_Cue))))

(fn ConstructionScript)

(fn SwitchCamera
  (bind _smartphone (Variables|Default|GetSmartphone))
  (bind _returnvalue (Audio|Components|Audio|IsPlaying _smartphone))
  (bind _returnvalue_2 (not _returnvalue))
  (if _returnvalue_2
    (if (and (Variables|Default|GetIsA) _returnvalue_2)
      (if (> (Variables|Default|Getbattery) 0.0)
        (CallFunction|SmartphoneAnimation "NewEnumerator0")
        (Variables|/Script/Engine.CharacterMovementComponent|SetMaxWalkSpeed (Variables|Character|GetCharacterMovement) (Variables|Default|GetwalkSpeed))
        (Variables|/Script/Engine.SceneCaptureComponent2D|SetTextureTarget (Variables|Default|GetSmartphoneCamera) "/Game/Blueprints/Sekine/Textures/SmartphoneCamera.SmartphoneCamera")
        (else
          (return)))
      (else
        (Variables|/Script/Engine.SceneCaptureComponent2D|SetTextureTarget (Variables|Default|GetSmartphoneCamera) 0)
        (CallFunction|SmartphoneAnimation "NewEnumerator1")))
    (bind _output_get (Variables|Default|SetIsA (not (Variables|Default|GetIsA))))
    (Variables|Default|SetholdCamera (not _output_get))))

(fn AddCellphoneHiddenActor
  (params (Actor :type Actor%20Object%20Reference))
  (Utilities|Array|Add (Variables|/Script/Engine.SceneCaptureComponent|GetHiddenActors (Variables|Default|GetSmartphoneCamera)) Actor))

(fn AddMainCameraHiddenActor
  (params (Actor :type Actor%20Object%20Reference))
  (Utilities|Array|Add (Variables|/Script/Engine.SceneCaptureComponent|GetHiddenActors (Variables|Default|GetMainCamera)) Actor))

(fn ChangeFOV
  (params (start :type Boolean))
  (bind _maincamera (Variables|Default|GetMainCamera))
  (if start
    (Variables|Default|SetFOVRun true)
    (Audio|PlaySoundatLocation "/Game/Sounds/SE/SystemSE/PlayerDiscovery_SE.PlayerDiscovery_SE" "0, 0, 0"))
  (if (Variables|Default|GetFOVRun)
    (bind _output_get (Variables|/Script/Engine.SceneCaptureComponent2D|SetFOVAngle _maincamera (+ (Variables|/Script/Engine.SceneCaptureComponent2D|GetFOVAngle _maincamera) (Variables|Default|GetFOVTmp))))
    (if (Variables|Default|GetFOVReverse)
      (if (> _output_get 9e+01)
        (Variables|/Script/Engine.SceneCaptureComponent2D|SetFOVAngle (Variables|Default|GetMainCamera) 9e+01)
        (Variables|Default|SetFOVReverse false)
        (Variables|Default|SetFOVRun false)
        (Variables|Default|SetFOVTmp (* -1 (Variables|Default|GetFOVTmp)) :!label _label))
      (elif (< _output_get 75.0)
        (Variables|Default|SetFOVReverse true)
        (goto _label)))))

(fn SmartphoneAnimation
  (params (AnimType :type AnimationType%20Enum :default "NewEnumerator4"))
  (switch Utilities|FlowControl|Switch|SwitchonAnimationType AnimType
    (:NewEnumerator0
      (Transformation|SetRelativeLocation (Variables|Default|GetSmartphone) "-40.000000,-25.000000,-95.000000" false true)
      (Development|SetHiddeninGame (Variables|Default|GetArm) false false)
      (Components|Animation|PlayAnimation (Variables|Default|GetSmartphone) "/Game/models/Taoki/camera_set/camera_set2_polySurface98_Anim.camera_set2_polySurface98_Anim" false)
      (Components|Animation|PlayAnimation (Variables|Default|GetArm) "/Game/models/Taoki/camera_set/camera_set2_polySurface99_Anim.camera_set2_polySurface99_Anim" false)
      (Variables|Default|SetbeforeAnim AnimType :!label _label))
    (:NewEnumerator1
      (Components|Animation|PlayAnimation (Variables|Default|GetSmartphone) "/Game/models/Taoki/camera_set/camera_set_modosu_sumaho2.camera_set_modosu_sumaho2" false)
      (Components|Animation|PlayAnimation (Variables|Default|GetArm) "/Game/models/Taoki/camera_set/camera_set_modosu_te.camera_set_modosu_te" false)
      (goto _label))
    (:NewEnumerator2
      (Transformation|SetRelativeLocation (Variables|Default|GetSmartphone) "10.000000,5.000000,-25.000000" false true)
      (Development|SetHiddeninGame (Variables|Default|GetArm) false false)
      (Components|Animation|PlayAnimation (Variables|Default|GetSmartphone) "/Game/models/Taoki/camera_set/sumaho_kazasu_sumaho.sumaho_kazasu_sumaho" false)
      (Components|Animation|PlayAnimation (Variables|Default|GetArm) "/Game/models/Taoki/camera_set/sumaho_kazasu_te.sumaho_kazasu_te" false)
      (goto _label))
    (:NewEnumerator3
      (if (Utilities|Enum|Equal(Enum) (Variables|Default|GetbeforeAnim) "NewEnumerator2")
        (Components|Animation|PlayAnimation (Variables|Default|GetSmartphone) "/Game/models/Taoki/camera_set/sumaho_kazasu_modosu_sumaho.sumaho_kazasu_modosu_sumaho" false)
        (Components|Animation|PlayAnimation (Variables|Default|GetArm) "/Game/models/Taoki/camera_set/sumaho_kazasu_modosu_te.sumaho_kazasu_modosu_te" false)
        (goto _label)))))