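; BP_Player is the player Blueprint, with a battery-powered camera and a game over level that loads on hitting an AlphaEnemy.
; Tick drains the battery while the camera is held, and an empty battery lowers the camera, removes its UI and hides the enemies.
; Battery changes update BP_MainHUD, found at BeginPlay.
; A short forward line trace each tick stores the actor in front, and overlap events track the overlapping actor.
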(event EventBeginPlay
  (bind _outactors (Actor|GetAllActorsOfClass "/Game/Blueprints/Sekine/BP_MainHUD.BP_MainHUD_C"))
  (for _array_element _outactors
    (bind _asbp_main_hud (Utilities|Casting|CastToBP_MainHUD _array_element))
    (Variables|Default|SetHUD _asbp_main_hud)))

(event Collision|EventActorBeginOverlap
  (params (OtherActor :type Actor%20Object%20Reference))
  (Variables|Default|SetOverlapActor OtherActor))

(event Collision|EventActorEndOverlap
  (params (OtherActor :type Actor%20Object%20Reference))
  (Variables|Default|SetOverlapActor 0))

(event EventTick
  (params (DeltaSeconds :type Float%20%28single-precision%29))
  (if (Variables|Default|GetHoldCamera)
    (CallFunction|SubBattery 2.0))
  (bind _actor (CallFunction|GetActionObject 1e+02))
  (Variables|Default|SetFront%20Actor _actor))

(event Collision|EventHit
  (params (MyComp :type Primitive%20Component%20Object%20Reference) (Other :type Actor%20Object%20Reference) (OtherComp :type Primitive%20Component%20Object%20Reference) (bSelfMoved :type Boolean) (HitLocation :type Vector :default "0, 0, 0") (HitNormal :type Vector :default "0, 0, 0") (NormalImpulse :type Vector :default "0, 0, 0") (Hit :type Hit%20Result%20Structure%20%28by%20ref%29))
  (Utilities|Casting|CastToAlphaEnemy Other)
  (Game|OpenLevel(byName) "GameOverLevel"))

(fn ConstructionScript)

(fn SubBattery
  (params (Value :type Float%20%28single-precision%29))
  (bind _output_get (Variables|Default|SetBattery (- (Variables|Default|GetBattery) (* Value (Utilities|Time|GetWorldDeltaSeconds)))))
  (if (< _output_get 1.0)
    (Variables|Default|SetBattery 0.0)
    (Variables|Default|SetHoldCamera false)
    (Widget|RemovefromParent (Variables|Default|GetCameraUI%20Class))
    (for _array_element (Variables|Default|GetEnemy)
      (Rendering|SetActorHiddenInGame _array_element true)))
  (Default|ChangeBatteryText (Variables|Default|GetHUD) (Math|Float|Truncate (Variables|Default|GetBattery))))

(fn AddBattery
  (params (Value :type Integer))
  (bind _output_get (Variables|Default|SetBattery (+ (Variables|Default|GetBattery) (Math|Conversions|ToFloat(Integer) Value))))
  (if (> _output_get 1e+02)
    (Variables|Default|SetBattery 1e+02))
  (Default|ChangeBatteryText (Variables|Default|GetHUD) (Math|Float|Truncate (Variables|Default|GetBattery))))

(fn GetActionObject
  (params (Length :type Float%20%28single-precision%29))
  (bind _capsulecomponent (Variables|Collision|GetCapsuleComponent))
  (bind _returnvalue (Transformation|GetWorldLocation _capsulecomponent))
  (bind _outhit (Collision|LineTraceByChannel _returnvalue (+ _returnvalue (* (Math|Vector|GetForwardVector _capsulecomponent) Length)) "TraceTypeQuery1" false 0 "None"))
  (return (.hitactor _outhit)))