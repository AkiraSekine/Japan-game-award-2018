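; BP_Switch is a switch the player operates via the smartphone, optionally requiring a key.
; Tick compares the player's ActionLocation with its position while the camera is not held, then plays the smartphone animation, sets the open button material and raises Action.
; Otherwise it clears Action and can show a missing-key UI hint, governed by a timer.
; At BeginPlay it caches the player and, if flagged invisible, hides itself from the main camera.
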(event EventBeginPlay
  (bind _outactors (Actor|GetAllActorsOfClass "/Game/Blueprints/Sekine/BP_MainPlayer.BP_MainPlayer_C"))
  (for _array_element _outactors
    (bind _asbp_main_player (Utilities|Casting|CastToBP_MainPlayer _array_element))
    (Variables|Default|Setplayer _asbp_main_player))
  (CallFunction|SetVisible (Variables|Default|GetisVisible)))

(event Collision|EventActorBeginOverlap
  (params (OtherActor :type Actor%20Object%20Reference)))

(event EventTick
  (params (DeltaSeconds :type Float%20%28single-precision%29))
  (if (and (Variables|Default|GetnoKeyTextDraw) (> (Variables|Default|GetnoKeyTextTime) 3.0))
    (Variables|Default|SetnoKeyTextTime (+ (Variables|Default|GetnoKeyTextTime) DeltaSeconds))
    (else
      (switch Utilities|FlowControl|Switch|SwitchonESlateVisibility (Widget|GetVisibility (Variables|/Game/Blueprints/Sekine/UI/MainCamera.MainCamera_C|GetKey (Variables|/Game/Blueprints/Sekine/BP_MainPlayer.BP_MainPlayer_C|GetMainUI (Variables|Default|Getplayer))))
        (:Visible
          (Widget|SetVisibility (Variables|/Game/Blueprints/Sekine/UI/MainCamera.MainCamera_C|GetKey (Variables|/Game/Blueprints/Sekine/BP_MainPlayer.BP_MainPlayer_C|GetMainUI (Variables|Default|Getplayer))) "Hidden")
          (Variables|Default|SetnoKeyTextDraw false))
        (:Collapsed
          _)
        (:Hidden
          _)
        (:HitTestInvisible
          _)
        (:SelfHitTestInvisible
          _))))
  (if (not (Variables|/Script/JGA2018Cpp.MainPlayer|GetholdCamera (Variables|Default|Getplayer)))
    (if (and (Math|Vector|Equal(Vector) (Variables|/Game/Blueprints/Sekine/BP_MainPlayer.BP_MainPlayer_C|GetactionLocation (Variables|Default|Getplayer)) (Transformation|GetActorLocation self) 0.0001) (or (and (Variables|Default|GetneedKey) (Variables|/Script/JGA2018Cpp.MainPlayer|GethaveKey (Variables|Default|Getplayer))) (not (Variables|Default|GetneedKey))))
      (if (not (Audio|Components|Audio|IsPlaying (Variables|/Game/Blueprints/Sekine/BP_MainPlayer.BP_MainPlayer_C|GetSmartphone (Variables|Default|Getplayer))))
        (Variables|Default|SetbackPlay false)
        (Utilities|FlowControl|DoOnce true :!label _label
          (:Completed
            (Default|SmartphoneAnimation (Variables|Default|Getplayer) "NewEnumerator3")
            (Rendering|Material|SetMaterial (Variables|Default|Getbutton) 0 "/Game/models/Takei/button/material/button_open.button_open")
            (Variables|Default|SetbackPlay true)
            (Variables|Default|Setaction true)))
        (elif (not (Variables|Default|GetbackPlay))
          (goto _label Reset)))
      (else
        (Variables|Default|Setaction false)
        (if (not (Audio|Components|Audio|IsPlaying (Variables|/Game/Blueprints/Sekine/BP_MainPlayer.BP_MainPlayer_C|GetSmartphone (Variables|Default|Getplayer))))
          (Default|SmartphoneAnimation (Variables|Default|Getplayer) "NewEnumerator3")
          (if (Variables|Default|GetneedKey)
            (Variables|Default|SetnoKeyTextTime 0.0)
            (Variables|Default|SetnoKeyTextDraw true)
            (Widget|SetVisibility (Variables|/Game/Blueprints/Sekine/UI/MainCamera.MainCamera_C|GetKey (Variables|/Game/Blueprints/Sekine/BP_MainPlayer.BP_MainPlayer_C|GetMainUI (Variables|Default|Getplayer))) "Visible")))))))

(fn ConstructionScript)

(fn SetVisible
  (params (newVisible :type Boolean))
  (if (not newVisible)
    (Default|AddMainCameraHiddenActor (Variables|Default|Getplayer) self)))