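; BP_Locker is a locker the player can move into and out of.
; Enter plays the Rokka animation, toggles the player's spotlight and starts the move.
; Tick lerps the player's location toward the locker interior or a point in front of it, chosen by Condition, and steers control rotation toward the locker's.
; On arrival within a small tolerance, movement stops and the player's Condition flips between Normal and Locker.
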(event EventBeginPlay
  (bind _outactors (Actor|GetAllActorsOfClass "/Game/Blueprints/Sekine/BP_MainPlayer.BP_MainPlayer_C"))
  (for _array_element _outactors
    (bind _asbp_main_player (Utilities|Casting|CastToBP_MainPlayer _array_element))
    (Variables|Default|SetPlayer _asbp_main_player)))

(event Collision|EventActorBeginOverlap
  (params (OtherActor :type Actor%20Object%20Reference)))

(event EventTick
  (params (DeltaSeconds :type Float%20%28single-precision%29))
  (bind _player (Variables|Default|GetPlayer))
  (if (and (Variables|Default|Getmoving) true)
    (switch Utilities|FlowControl|Switch|SwitchonEPlayerCondition (Variables|/Script/JGA2018Cpp.MainPlayer|Getcondition (Variables|Default|GetPlayer))
      (:Normal
        (Transformation|SetActorLocation (Variables|Default|GetPlayer) (Math|Vector|Lerp(Vector) (Transformation|GetActorLocation (Variables|Default|GetPlayer)) (+ (Transformation|GetActorLocation) "0, 0,100.000000") (* (Utilities|Time|GetWorldDeltaSeconds) 5.0)) false false)
        (Pawn|SetControlRotation (Game|GetPlayerController 0) (Math|Rotator|Lerp(Rotator) (Transformation|GetActorRotation (Variables|Default|GetPlayer)) (Transformation|GetActorRotation) (* (Utilities|Time|GetWorldDeltaSeconds) 5.0)))
        (if (Math|Vector|Equal(Vector) (Transformation|GetActorLocation (Variables|Default|GetPlayer)) (+ (Transformation|GetActorLocation) "0, 0,100.000000") 0.1)
          (Variables|Default|Setmoving false :!label _label)
          (switch Utilities|FlowControl|Switch|SwitchonEPlayerCondition (Variables|/Script/JGA2018Cpp.MainPlayer|Getcondition (Variables|Default|GetPlayer))
            (:Normal
              (Variables|/Script/JGA2018Cpp.MainPlayer|Setcondition _player "Locker"))
            (:Locker
              (Variables|/Script/JGA2018Cpp.MainPlayer|Setcondition _player "Normal")))))
      (:Locker
        (Transformation|SetActorLocation (Variables|Default|GetPlayer) (Math|Vector|Lerp(Vector) (Transformation|GetActorLocation (Variables|Default|GetPlayer)) (+ (Transformation|GetActorLocation) (* (Math|Vector|GetForwardVector (Variables|Default|GetBox)) 125.0) "0,0,90.000000") (* (Utilities|Time|GetWorldDeltaSeconds) 5.0)) false false)
        (Pawn|SetControlRotation (Game|GetPlayerController 0) (Math|Rotator|Lerp(Rotator) (Transformation|GetActorRotation (Variables|Default|GetPlayer)) (Transformation|GetActorRotation) (* (Utilities|Time|GetWorldDeltaSeconds) 5.0)))
        (if (Math|Vector|Equal(Vector) (Transformation|GetActorLocation (Variables|Default|GetPlayer)) (+ (Transformation|GetActorLocation) (* (Math|Vector|GetForwardVector (Variables|Default|GetBox)) 125.0) "0,0,90.000000") 0.1)
          (goto _label))))))

(fn ConstructionScript)

(fn Enter
  (bind _player (Variables|Default|GetPlayer))
  (bind _spotlight (Variables|/Game/Blueprints/Sekine/BP_MainPlayer.BP_MainPlayer_C|GetSpotLight _player))
  (Variables|Default|Setmoving true)
  (Components|Animation|PlayAnimation (Variables|Default|Getrokka) 0 false)
  (switch Utilities|FlowControl|Switch|SwitchonEPlayerCondition (Variables|/Script/JGA2018Cpp.MainPlayer|Getcondition (Variables|Default|GetPlayer))
    (:Normal
      (Development|SetHiddeninGame _spotlight true false))
    (:Locker
      (Development|SetHiddeninGame _spotlight false false))))