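; BP_Door is a sliding door that opens for overlapping actors when CanOpen is set, with frame and door materials showing that state.
; Overlaps update a counter and play the MoveDoor timeline, which lerps the door sideways and reverses once the counter reaches zero.
; The timeline plays even when locked, but only moves the door if CanOpen.
; Tick polls an optional Switch and unlocks the door when its Action is true.
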(event EventBeginPlay
  (Transformation|SetRelativeLocation (Variables|Default|GetDoor) "0, 0, 0" false true)
  (CallFunction|ChangeCanOpen (Variables|Default|GetcanOpen)))

(event Collision|EventActorBeginOverlap
  (params (OtherActor :type Actor%20Object%20Reference))
  (CallFunction|CountUp (Variables|Default|GetOverlapActorsCount))
  (bind _open (Timeline|Move%20Door Play)
    (:Update
      (if (Variables|Default|GetcanOpen)
        (Transformation|SetRelativeLocation (Variables|Default|GetDoor) (Math|Vector|Lerp(Vector) "0, 0, 0" "0,250.000000,0.000000" _open) false false)))))

(event Collision|EventActorEndOverlap
  (params (OtherActor :type Actor%20Object%20Reference))
  (CallFunction|CountDown (Variables|Default|GetOverlapActorsCount))
  (if (<= (Variables|Default|GetOverlapActorsCount) 0)
    (bind _open (Timeline|Move%20Door Reverse)
      (:Update
        (if (Variables|Default|GetcanOpen)
          (Transformation|SetRelativeLocation (Variables|Default|GetDoor) (Math|Vector|Lerp(Vector) "0, 0, 0" "0,250.000000,0.000000" _open) false false))))))

(event EventTick
  (params (DeltaSeconds :type Float%20%28single-precision%29))
  (if (!= (Variables|Default|Getswitch) 0)
    (if (Variables|/Game/Blueprints/Sekine/BP_Switch.BP_Switch_C|Getaction (Variables|Default|Getswitch))
      (CallFunction|ChangeCanOpen true))))

(fn ConstructionScript)

(fn ChangeCanOpen
  (params (newCanOpen :type Boolean))
  (bind _output_get (Variables|Default|SetcanOpen newCanOpen))
  (if _output_get
    (Rendering|Material|SetMaterial (Variables|Default|GetFrame) 0 "/Game/models/Takei/door/Material/door_OK.door_OK")
    (else
      (Rendering|Material|SetMaterial (Variables|Default|GetFrame) 0 "/Game/models/Takei/door/Material/door_BAD.door_BAD"))))

(fn CountUp
  (params (Data :type Integer%20%28by%20ref%29))
  (|SetBy-RefVar Data (+ Data 1)))

(fn CountDown
  (params (Data :type Integer%20%28by%20ref%29))
  (|SetBy-RefVar Data (- Data 1)))