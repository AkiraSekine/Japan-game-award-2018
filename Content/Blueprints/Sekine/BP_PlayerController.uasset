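; Player controller for BP_Player, handling movement, sprint, look and a toggled handheld video camera that reveals otherwise hidden AlphaEnemy actors.
; BeginPlay caches and hides the enemies; the camera toggle shows its UI, unhides them and blocks sprinting.
; One player Condition state disables movement and pitch, redirecting yaw to the overlapped actor's camera within a narrow range.
; Action flags interaction, calls AddBattery at chargers and destroys Tips actors in front.
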(event EventBeginPlay
  (bind _returnvalue (UserInterface|CreateWidget "/Game/Blueprints/Sekine/BP_MainUI.BP_MainUI_C"))
  (Variables|Default|SetCamera%20UI%20Class _returnvalue)
  (bind _outactors (Actor|GetAllActorsOfClass "/Game/Blueprints/Reito/Enemy/AI_test/AlphaEnemy.AlphaEnemy_C"))
  (for (_array_element _array_index) _outactors
    (bind _asalpha_enemy (Utilities|Casting|CastToAlphaEnemy _array_element))
    (Utilities|Array|Add (Variables|Default|GetEnemy) _asalpha_enemy)
    (Rendering|SetActorHiddenInGame (Utilities|Array|Get(acopy) (Variables|Default|GetEnemy) _array_index) true))
  (bind _asbp_player (Utilities|Casting|CastToBP_Player (Pawn|GetControlledPawn)))
  (Variables|Default|SetBP%20Player _asbp_player))

(event EventTick
  (params (DeltaSeconds :type Float%20%28single-precision%29)))

(event Input|ActionEvents|InputActionCamera
  (params (Key :type Key%20Structure))
  (bind _camera_ui_class (Variables|Default|GetCamera%20UI%20Class))
  ;[1 1 1] Video camera
  (:Pressed
    (bind _isa (Utilities|FlowControl|FlipFlop)
      (:A
        (UserInterface|Viewport|AddtoViewport _camera_ui_class 0)
        (Variables|Default|SetWalk%20Speed (Variables|Default|GetDefault%20Walk%20Speed)))
      (:B
        (Widget|RemovefromParent _camera_ui_class)))
    (bind _output_get (Variables|/Game/Blueprints/Sekine/BP_Player.BP_Player_C|SetHoldCamera (Variables|Default|GetBP%20Player) _isa))
    (for _array_element (Variables|Default|GetEnemy)
      (Rendering|SetActorHiddenInGame _array_element (not _output_get)))))

(event Input|ActionEvents|InputActionSprint
  (params (Key :type Key%20Structure))
  (bind _bp_player (Variables|Default|GetBP%20Player))
  (bind _condition (Variables|/Game/Blueprints/Sekine/BP_Player.BP_Player_C|GetCondition _bp_player))
  (bind _holdcamera (Variables|/Game/Blueprints/Sekine/BP_Player.BP_Player_C|GetHoldCamera _bp_player))
  (bind _returnvalue (not _holdcamera))
  (bind _returnvalue_2 (Utilities|Enum|NotEqual(Enum) _condition "NewEnumerator1"))
  (bind _returnvalue_3 (and _returnvalue _returnvalue_2))
  ;[1 1 1] Move
  (:Pressed
    (if _returnvalue_3
      (Variables|Default|SetWalk%20Speed (* (Variables|Default|GetDefault%20Walk%20Speed) 1.5))))
  (:Released
    (if _returnvalue_3
      (Variables|Default|SetWalk%20Speed (Variables|Default|GetDefault%20Walk%20Speed)))))

(event Input|ActionEvents|InputActionAction
  (params (Key :type Key%20Structure))
  (bind _bp_player (Variables|Default|GetBP%20Player))
  (bind _bp_player_2 (Variables|Default|GetBP%20Player))
  (bind _front_actor (Variables|/Game/Blueprints/Sekine/BP_Player.BP_Player_C|GetFront%20Actor _bp_player))
  ;[1 1 1] アクション
  (:Pressed
    (Variables|/Game/Blueprints/Sekine/BP_Player.BP_Player_C|SetIs%20Action _bp_player_2 true)
    (Utilities|Casting|CastToBP_Charger _front_actor
      (:then
        (Default|AddBattery (Variables|Default|GetBP%20Player)))
      (:CastFailed
        _))
    (bind _astips (Utilities|Casting|CastToTips _front_actor))
    (Actor|DestroyActor _astips))
  (:Released
    (Variables|/Game/Blueprints/Sekine/BP_Player.BP_Player_C|SetIs%20Action _bp_player_2 false)))

(event Input|AxisEvents|InputAxisTurn
  (params (AxisValue :type Float%20%28single-precision%29))
  (bind _returnvalue (Utilities|Time|GetWorldDeltaSeconds))
  (bind _yaw_speed (Variables|Default|GetYaw%20Speed))
  (bind _bp_player (Variables|Default|GetBP%20Player))
  (bind _returnvalue_2 (* AxisValue _returnvalue _yaw_speed))
  (bind _overlapactor (Variables|/Game/Blueprints/Sekine/BP_Player.BP_Player_C|GetOverlapActor _bp_player))
  (bind _returnvalue_3 (Actor|GetComponentbyClass _overlapactor "/Script/Engine.CameraComponent"))
  (bind _returnvalue_4 (Transformation|GetRelativeTransform _returnvalue_3))
  (bind _returnvalue_5 (> (.yaw (.rotation _returnvalue_4)) -1e+01))
  (bind _returnvalue_6 (< (.yaw (.rotation _returnvalue_4)) 1e+01))
  (bind _returnvalue_7 (and _returnvalue_5 _returnvalue_6))
  ;[1 1 1] Camera
  (if (Utilities|Enum|NotEqual(Enum) (Variables|/Game/Blueprints/Sekine/BP_Player.BP_Player_C|GetCondition (Variables|Default|GetBP%20Player)) "NewEnumerator1")
    (Pawn|Input|AddControllerYawInput (Variables|Default|GetBP%20Player) _returnvalue_2)
    (elif _returnvalue_7
      (Transformation|AddLocalRotation _returnvalue_3 (Math|Rotator|MakeRotator 0.0 0.0 _returnvalue_2) false false)
      (if (not _returnvalue_7)
        (Transformation|AddLocalRotation _returnvalue_3 (Math|Rotator|MakeRotator 0.0 0.0 (* -1 _returnvalue_2)) false false)))))

(event Input|AxisEvents|InputAxisMoveForward
  (params (AxisValue :type Float%20%28single-precision%29))
  ;[1 1 1] Move
  (if (Utilities|Enum|NotEqual(Enum) (Variables|/Game/Blueprints/Sekine/BP_Player.BP_Player_C|GetCondition (Variables|Default|GetBP%20Player)) "NewEnumerator1")
    (Pawn|Input|AddMovementInput (Variables|Default|GetBP%20Player) (Math|Vector|GetForwardVector (Variables|/Script/Engine.Actor|GetRootComponent (Variables|Default|GetBP%20Player))) (* AxisValue (Variables|Default|GetWalk%20Speed)) false)))

(event Input|AxisEvents|InputAxisMoveRight
  (params (AxisValue :type Float%20%28single-precision%29))
  ;[1 1 1] Move
  (if (Utilities|Enum|NotEqual(Enum) (Variables|/Game/Blueprints/Sekine/BP_Player.BP_Player_C|GetCondition (Variables|Default|GetBP%20Player)) "NewEnumerator1")
    (Pawn|Input|AddMovementInput (Variables|Default|GetBP%20Player) (Math|Vector|GetRightVector (Variables|/Script/Engine.Actor|GetRootComponent (Variables|Default|GetBP%20Player))) (* AxisValue (Variables|Default|GetWalk%20Speed)) false)))

(event Input|AxisEvents|InputAxisLookUp
  (params (AxisValue :type Float%20%28single-precision%29))
  ;[1 1 1] Camera
  (if (Utilities|Enum|NotEqual(Enum) (Variables|/Game/Blueprints/Sekine/BP_Player.BP_Player_C|GetCondition (Variables|Default|GetBP%20Player)) "NewEnumerator1")
    (Pawn|Input|AddControllerPitchInput (Variables|Default|GetBP%20Player) (* AxisValue (Utilities|Time|GetWorldDeltaSeconds) (Variables|Default|GetPitch%20Speed)))))

(fn ConstructionScript)