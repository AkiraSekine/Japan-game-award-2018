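; BP_Key is a key actor that can be given to the main player.
; GiveKey flags the player as holding a key and updates the player's menu.
; BeginPlay caches the player, and once the key is given, Tick waits for the smartphone to stop playing, then destroys the key component and triggers a smartphone animation.
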(event EventBeginPlay
  (bind _outactors (Actor|GetAllActorsOfClass "/Game/Blueprints/Sekine/BP_MainPlayer.BP_MainPlayer_C"))
  (for _array_element _outactors
    (bind _asbp_main_player (Utilities|Casting|CastToBP_MainPlayer _array_element))
    (Variables|Default|Setplayer _asbp_main_player)))

(event Collision|EventActorBeginOverlap
  (params (OtherActor :type Actor%20Object%20Reference)))

(event EventTick
  (params (DeltaSeconds :type Float%20%28single-precision%29))
  (if (and (Variables|Default|Getis%20Gave) (not (Audio|Components|Audio|IsPlaying (Variables|/Game/Blueprints/Sekine/BP_MainPlayer.BP_MainPlayer_C|GetSmartphone (Variables|Default|Getplayer)))))
    (Components|DestroyComponent (Variables|Default|GetKey))
    (Default|SmartphoneAnimation (Variables|Default|Getplayer) "NewEnumerator3")
    (Variables|Default|Setis%20Gave false)))

(fn ConstructionScript)

(fn GiveKey
  (params (Player :type BP%20Main%20Player%20Object%20Reference))
  (Variables|/Script/JGA2018Cpp.MainPlayer|SethaveKey Player true)
  (Variables|Default|Setis%20Gave true)
  (Default|KeySet (Variables|/Game/Blueprints/Sekine/BP_MainPlayer.BP_MainPlayer_C|GetMenu Player)))