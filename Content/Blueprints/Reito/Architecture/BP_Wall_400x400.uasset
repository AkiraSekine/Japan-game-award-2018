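; Wall actor that turns into a door mesh while the player holds the camera and the wall was recently rendered, otherwise showing the 400x400 wall mesh.
; On BeginPlay it finds BP_MainPlayer and spawns a BP_NoColliderWall at its own transform.
; It registers that copy as hidden from the cellphone and itself as hidden from the main camera, so each view sees a different actor.
; Tick drives the mesh swap.
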(event EventBeginPlay
  ;[1 1 1] 生成&破棄処理
  (Components|StaticMesh|SetStaticMesh (Variables|Default|GetSM_Wall_400x400) "/Game/Blueprints/Reito/Architecture/SM_Wall_400x400.SM_Wall_400x400")
  (bind _outactors (Actor|GetAllActorsOfClass "/Game/Blueprints/Sekine/BP_MainPlayer.BP_MainPlayer_C"))
  (for _array_element _outactors
    (bind _asbp_main_player (Utilities|Casting|CastToBP_MainPlayer _array_element))
    (Variables|Default|SetPlayers_bool _asbp_main_player))
  (bind _returnvalue (Game|SpawnActorfromClass "/Game/Blueprints/Reito/Architecture/BP_NoColliderWall.BP_NoColliderWall_C" (Transformation|GetActorTransform) "Undefined" 0 0))
  (Default|AddCellphoneHiddenActor (Variables|Default|GetPlayers_bool) _returnvalue)
  (Default|AddMainCameraHiddenActor (Variables|Default|GetPlayers_bool) self))

(event Collision|EventActorBeginOverlap
  (params (OtherActor :type Actor%20Object%20Reference)))

(event EventTick
  (params (DeltaSeconds :type Float%20%28single-precision%29))
  ;[1 1 1] 生成&破棄処理
  (if (Variables|/Script/JGA2018Cpp.MainPlayer|GetholdCamera (Variables|Default|GetPlayers_bool))
    (if (Class|Actor|WasRecentlyRendered 0.2)
      (Components|StaticMesh|SetStaticMesh (Variables|Default|GetSM_Wall_400x400) "/Game/Blueprints/Reito/Architecture/SM_Door.SM_Door")
      (else
        (Components|StaticMesh|SetStaticMesh (Variables|Default|GetSM_Wall_400x400) "/Game/Blueprints/Reito/Architecture/SM_Wall_400x400.SM_Wall_400x400" :!label _label)))
    (else
      (goto _label))))

(fn ConstructionScript)