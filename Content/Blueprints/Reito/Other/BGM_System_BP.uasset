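; BGM_System_BP is a background music actor that starts the stage track on BeginPlay and caches the BP_MainPlayer as Action.
; The N_BGM playback-percent callback accumulates delta seconds into BGMTime and prints it, then checks the player's Action flag without acting on it.
; Logic for swapping to a reversed track at a mirrored time offset is disconnected, so it never runs.
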(event OnAudioPlaybackPercent(N_BGM)
  (params (PlayingSoundWave :type Sound%20Wave%20Object%20Reference) (PlaybackPercent :type Float%20%28single-precision%29))
  (bind _output_get (Variables|Default|SetBGM_time (+ (Utilities|Time|GetWorldDeltaSeconds) (Variables|Default|GetBGM_time))))
  (Development|PrintString (Utilities|String|ToString(Float) _output_get))
  (if (Variables|/Script/JGA2018Cpp.MainPlayer|Getaction (Variables|Default|GetAction))
    _))

(event OnAudioPlaybackPercent(Reverse_BGM)
  (params (PlayingSoundWave :type Sound%20Wave%20Object%20Reference) (PlaybackPercent :type Float%20%28single-precision%29)))

(event EventBeginPlay
  (Audio|Components|Audio|Play (Variables|Default|GetN_BGM) 0.0)
  (bind _outactors (Actor|GetAllActorsOfClass "/Game/Blueprints/Sekine/BP_MainPlayer.BP_MainPlayer_C"))
  (for _array_element _outactors
    (bind _asbp_main_player (Utilities|Casting|CastToBP_MainPlayer _array_element))
    (Variables|Default|SetAction _asbp_main_player)))

(event Collision|EventActorBeginOverlap
  (params (OtherActor :type Actor%20Object%20Reference)))

(event EventTick
  (params (DeltaSeconds :type Float%20%28single-precision%29))
  (if (>= (Variables|Default|GetBGM_time) 0.0)
    _))

(fn ConstructionScript)