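; BP_Locker is a locker the player can step into and out of.
; It tracks the overlapping actor and, on Tick, detects a fresh press of BP_Player's IsAction to call Enter when the locker is the player's FrontActor.
; Enter toggles the player's Condition: entering switches the view target to the locker's camera; exiting teleports the player just in front, facing outward, and returns the view.
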(event EventBeginPlay)

(event Collision|EventActorBeginOverlap
  (params (OtherActor :type Actor%20Object%20Reference))
  (Variables|Default|SetOverlap%20Actor OtherActor))

(event EventTick
  (params (DeltaSeconds :type Float%20%28single-precision%29))
  (bind _asbp_player (Utilities|Casting|CastToBP_Player (Variables|Default|GetOverlap%20Actor)))
  (if (and (Variables|/Game/Brueprints/Sekine/BP_Player.BP_Player_C|GetIs%20Action _asbp_player) (not (Variables|Default|GetActionBefore)))
    (CallFunction|Enter))
  (Variables|Default|SetActionBefore (Variables|/Game/Brueprints/Sekine/BP_Player.BP_Player_C|GetIs%20Action _asbp_player)))

(event Collision|EventActorEndOverlap
  (params (OtherActor :type Actor%20Object%20Reference))
  (Variables|Default|SetOverlap%20Actor 0))

(event Input|ActionEvents|InputActionAction
  (params (Key :type Key%20Structure)))

(fn ConstructionScript)

(fn Enter
  (bind _asbp_player (Utilities|Casting|CastToBP_Player (Variables|Default|GetOverlap%20Actor)))
  (bind _output_get (LocalVariables|SetCastedPlayer _asbp_player))
  (if (== (Variables|/Game/Brueprints/Sekine/BP_Player.BP_Player_C|GetFront%20Actor (LocalVariables|GetCastedPlayer)) self)
    (switch Utilities|FlowControl|Switch|SwitchonPlayerCondition (Variables|/Game/Brueprints/Sekine/BP_Player.BP_Player_C|GetCondition _output_get)
      (:NewEnumerator0
        (Variables|/Game/Brueprints/Sekine/BP_Player.BP_Player_C|SetCondition (LocalVariables|GetCastedPlayer) "NewEnumerator1")
        (Transformation|SetRelativeRotation (Variables|Default|GetCamera) "0, 0, 0" false false)
        (Game|Player|SetViewTargetwithBlend (Game|GetPlayerController 0) self 0.0 "VTBlend_Linear" 0.0 false))
      (:NewEnumerator1
        (Transformation|SetActorLocation (LocalVariables|GetCastedPlayer) (+ (* (Transformation|GetActorForwardVector) 5e+01) (Transformation|GetActorLocation)) false true)
        (Transformation|SetActorRotation (Game|Player|GetPlayerPawn 0) (Transformation|GetActorRotation) true)
        (Variables|/Game/Brueprints/Sekine/BP_Player.BP_Player_C|SetCondition (LocalVariables|GetCastedPlayer) "NewEnumerator0")
        (Game|Player|SetViewTargetwithBlend (Game|GetPlayerController 0) (Variables|Default|GetOverlap%20Actor) 0.0 "VTBlend_Linear" 0.0 false)))))