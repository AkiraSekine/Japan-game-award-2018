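; BP_MainHUD is a HUD Blueprint that draws the player's battery percentage and a key indicator on screen.
; On BeginPlay it finds the BP_Player actor and caches a reference to it.
; DrawHUD draws the Battery string each frame, adding a "Key" label while the player's HaveKey flag is set.
; ChangeBatteryText formats a given value as a percentage into that Battery string.
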(event EventBeginPlay
  (bind _outactors (Actor|GetAllActorsOfClass "/Game/Brueprints/Sekine/BP_Player.BP_Player_C"))
  (for _array_element _outactors
    (bind _asbp_player (Utilities|Casting|CastToBP_Player _array_element))
    (Variables|Default|SetPlayer _asbp_player)))

(event Collision|EventActorBeginOverlap
  (params (OtherActor :type Actor%20Object%20Reference)))

(event EventTick
  (params (DeltaSeconds :type Float%20%28single-precision%29)))

(event EventDrawHUD
  (params (SizeX :type Integer) (SizeY :type Integer))
  (HUD|DrawText (Variables|Default|GetBattery) "(R=0,G=0,B=0,A=1)" 5e+01 5e+01 "/Game/Fonts/BatteryFont.BatteryFont" 1.0 false)
  (if (Variables|/Game/Brueprints/Sekine/BP_Player.BP_Player_C|GetHave%20Key (Variables|Default|GetPlayer))
    (HUD|DrawText "Key" "(R=0,G=0,B=0,A=1)" 2e+02 5e+01 "/Game/Fonts/BatteryFont.BatteryFont" 1.0 false)))

(fn ConstructionScript)

(fn ChangeBatteryText
  (params (Value :type Integer))
  (Variables|Default|SetBattery (Utilities|String|Append (Utilities|String|ToString(Integer) Value) "%")))