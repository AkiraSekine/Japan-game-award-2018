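; BP_Wall_400x400 is a wall actor that appears as a door wall while the player holds the camera and the wall is on screen.
; On BeginPlay it finds and stores a reference to BP_Player.
; Every Tick it checks HoldCamera and WasRecentlyRendered to swap its static mesh between the door and plain wall variants.
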(event EventBeginPlay
  ;[1 1 1] 生成&破棄処理
  (bind _outactors (Actor|GetAllActorsOfClass "/Game/Brueprints/Sekine/BP_Player.BP_Player_C"))
  (for _array_element _outactors
    (bind _asbp_player (Utilities|Casting|CastToBP_Player _array_element))
    (Variables|Default|SetPlayers_bool _asbp_player)))

(event Collision|EventActorBeginOverlap
  (params (OtherActor :type Actor%20Object%20Reference)))

(event EventTick
  (params (DeltaSeconds :type Float%20%28single-precision%29))
  ;[1 1 1] 生成&破棄処理
  (if (Variables|/Game/Brueprints/Sekine/BP_Player.BP_Player_C|GetHoldCamera (Variables|Default|GetPlayers_bool))
    (if (Class|Actor|WasRecentlyRendered 0.2)
      (Components|StaticMesh|SetStaticMesh (Variables|Default|GetSM_Wall_400x400) "/Game/Brueprints/Reito/Architecture/SM_Wall_Door_400x400.SM_Wall_Door_400x400")
      (else
        (Components|StaticMesh|SetStaticMesh (Variables|Default|GetSM_Wall_400x400) "/Game/Brueprints/Reito/Architecture/SM_Wall_400x400.SM_Wall_400x400" :!label _label)))
    (else
      (goto _label))))

(fn ConstructionScript)